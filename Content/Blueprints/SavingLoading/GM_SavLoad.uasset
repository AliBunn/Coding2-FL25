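; GM_SavLoad is a Game Mode that handles saving and loading player stats through an SG_PlayerStats save object in the PlayerSave slot.
; On BeginPlay it loads the existing save and copies the saved Stamina onto the BP_ThirdPersonCharacter, or creates a fresh save object if none exists.
; SavePlayerStats writes the held save object to the slot without reading values from the character, and prints whether the write succeeded.
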(event Custom|Load%20Player%20Stats
  (bind _returnvalue (SaveGame|DoesSaveGameExist "PlayerSave"))
  (if _returnvalue
    (bind _returnvalue_2 (SaveGame|LoadGamefromSlot "PlayerSave"))
    (bind _assg_player_stats (Utilities|Casting|CastToSG_PlayerStats _returnvalue_2))
    (Variables|Default|SetSG_PlayerStats _assg_player_stats)
    (bind _asbp_third_person_character (Utilities|Casting|CastToBP_ThirdPersonCharacter (Game|GetPlayerCharacter 0)))
    (Variables|/Game/ThirdPerson/Blueprints/BP_ThirdPersonCharacter.BP_ThirdPersonCharacter_C|SetStamina _asbp_third_person_character (Variables|/Game/Blueprints/SavingLoading/SG_PlayerStats.SG_PlayerStats_C|GetStamina (Variables|Default|GetSG_PlayerStats))) ; The Player's Stamina
    (Development|PrintString "PlayerStats have been loaded." true true "(R=1.000000,G=0.064348,B=0.000000,A=1.000000)" 8.0)
    (else
      (bind _returnvalue_3 (SaveGame|CreateSaveGameObject "/Game/Blueprints/SavingLoading/SG_PlayerStats.SG_PlayerStats_C"))
      (Variables|Default|SetSG_PlayerStats _returnvalue_3) ; set this variable so that the \nPlayer can edit these values
    )))

(event Custom|Save%20Player%20Stats
  (bind _returnvalue (SaveGame|SaveGametoSlot (Variables|Default|GetSG_PlayerStats) "PlayerSave"))
  (if _returnvalue
    (Development|PrintText "Player Stats Written to Save Game File" true true "(R=0.321655,G=1.000000,B=0.013734,A=1.000000)" 5.0)
    (else
      (Development|PrintText "Player Stats Could Not be Written to Save Game File" true true "(R=1.000000,G=0.000528,B=0.043477,A=1.000000)" 5.0))))

(event EventBeginPlay
  (Development|PrintString "Loading the SavLoad Game Mode" true true "(R=1.000000,G=0.244464,B=0.000000,A=1.000000)" 1e+01)
  (CallFunction|LoadPlayerStats))

(fn ConstructionScript)